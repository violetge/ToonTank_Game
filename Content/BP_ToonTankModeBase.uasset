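; Game mode Blueprint for a Toon Tank game that shows the start screen when play begins.
; BeginPlay calls StartGame, which prints a debug message, creates the WBP_Start widget and adds it to the viewport.
; A Countdown event decrements a number and writes it to the widget's text, but its looping one-second timer setup is disconnected and never runs.
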(event Custom|Start%20Game
  (Development|PrintString "Start")
  (bind _returnvalue (UserInterface|CreateWidget "/Game/WBP_Start.WBP_Start_C"))
  (bind _output_get (Variables|Default|SetNewVar _returnvalue))
  (UserInterface|Viewport|AddtoViewport _output_get 0))

(event Custom|Countdown
  ;[1 1 1] 也是一种倒计时的实现 不过只能显示纯时间
  (if (> (Variables|Default|GetCount%20down%20Number) 0.0)
    (bind _result (Math|Float|DecrementFloat (Variables|Default|GetCount%20down%20Number))
      (:%20%20
        (bind _output_get (Variables|Default|SetCount%20down%20Number _result))
        (Rendering|Components|TextRender|SetText (Variables|/Game/WBP_Start.WBP_Start_C|GetCountdown_Numnber (Variables|Default|GetNewVar)) (Utilities|Text|ToText(Float) _output_get "HalfToEven"))))))

(event EventBeginPlay
  (CallFunction|StartGame))

(event EventTick
  (params (DeltaSeconds :type Float%20%28single-precision%29)))

(fn ConstructionScript)